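; Vegetable is an actor that grows through visual stages over time by swapping its static mesh.
; BeginPlay sets the first mesh, then a Tick-driven DoOnce with a one-second Delay increments and prints a timer.
; When the timer equals the current step's time in StepsTimes, NextStep applies the next mesh from StepsMeshes.
; The DoOnce resets after each second until the last mesh is reached, which stops the timer.
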(event `self.ReceiveBeginPlay`
  (`StaticMeshComponent.SetStaticMesh` (`self.StaticMesh`) (`|GetArrayItem` (`self.stepsMeshes`))))

(event `self.ReceiveTick`
  (params (DeltaSeconds :type "Float (single-precision)"))
  (bind _timer (`self.timer`))
  (`/Engine/EditorBlueprintResources/StandardMacros.DoOnce` false :!label _label
    (:`Completed`
      (`KismetSystemLibrary.Delay` 1.0)
      (set `self.timer` (+ _timer 1.0))
      (`KismetSystemLibrary.PrintString` (`KismetStringLibrary.Conv_DoubleToString` _timer))
      (if (== (`self.timer`) (`|GetArrayItem` (`self.stepsTimes`) (`self.step`)))
        (`self.nextStep`)
        (if (not (`self.fullyGrown`))
          (goto _label :!via `Reset`))
        (else
          (goto _label :!via `Reset`))))))

(fn `fullyGrown`
  (returns (ReturnValue :type Boolean))
  (return (== (`KismetArrayLibrary.Array_Length` (`self.stepsMeshes`)) (+ (`self.step`) 1))))

(fn `nextStep`
  (bind _step (`self.step`))
  (`/Engine/EditorBlueprintResources/StandardMacros.IncrementInt` _step
    (:`  `
      (`StaticMeshComponent.SetStaticMesh` (`self.StaticMesh`) (`|GetArrayItem` (`self.stepsMeshes`) _step)))))

(fn `UserConstructionScript`)