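; Utility Blueprint functions for fetching the player character and looking up item data.
; GetCharacter returns the first player's character cast to MainCharacter.
; GetItemInfoByName reads a row from ItemsInfoDataTable and reports whether it was found.
; GetItemInfoByItem wraps that lookup using the item's Name, returning the row info without a found flag.
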(fn `GetCharacter`
  (returns (character :type "/Game/Character/MainCharacter Object Reference"))
  (bind _asmain_character (cast `/Game/Character/MainCharacter` (`GameplayStatics.GetPlayerCharacter` null)))
  (return _asmain_character))

(fn `GetItemInfoByItem`
  (params (item :type "/Game/StructuresAndEnums/ItemWithQuantity Structure"))
  (returns (itemInfo :type "/Game/StructuresAndEnums/ItemInfo Structure"))
  (bind (_found _iteminfo) (`self.GetItemInfoByName` (`.name_7_078CAAEF4FECD75C7C54FD8068C5F96D` (break `/Game/StructuresAndEnums/ItemWithQuantity` item))))
  (if _found
    (return _iteminfo)
    (else
      (return))))

(fn `GetItemInfoByName`
  (params (name :type Name))
  (returns (found :type Boolean) (itemInfo :type "/Game/StructuresAndEnums/ItemInfo Structure"))
  (bind _returnvalue (`|GetDataTableRow` "/Game/StructuresAndEnums/ItemsInfoDataTable.ItemsInfoDataTable" name)
    (:`then`
      (return true _returnvalue))
    (:`RowNotFound`
      (return false))))