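; DirtRectangle is an actor Blueprint that lays out a flat rectangular grid of Dirt actors.
; Its construction script runs nested loops over Width and Height, adding a Child Actor Component of the Dirt class at each cell, spaced by DirtSize along X and Y.
; The event graph holds only disabled placeholder events, so all behavior happens at construction.
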(fn `UserConstructionScript`
  (for _index (range (+ (`self.width`) 1))
    (for _index_2 (range (+ (`self.height`) 1))
      (bind _returnvalue (`AddComponent|NODE_AddChildActorComponent-0` :`RelativeTransform` (`KismetMathLibrary.MakeTransform` (`KismetMathLibrary.MakeVector` (* _index (`self.dirtSize`)) (* _index_2 (`self.dirtSize`))) (struct) (1.0 1.0 1.0))))
      (`ChildActorComponent.SetChildActorClass` _returnvalue "/Game/Blueprints/dirt.dirt_C"))))